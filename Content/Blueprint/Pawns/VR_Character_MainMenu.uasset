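; VR pawn for the main menu that moves along camera direction and operates widgets with a laser pointer from either hand.
; BeginPlay sets the tracking origin per headset and offsets the VR origin by character height.
; Each Tick, a short object trace from the selected hand toggles its interaction component and red line and positions its dot.
; Triggers click while a widget is hit, otherwise they choose the pointing hand.
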(event `self.ReceiveBeginPlay`
  ;[1 1 1] FloorLevel
  (switch `name` (`HeadMountedDisplayFunctionLibrary.GetHMDDeviceName`)
    (:`Oculus Rift`
      (`HeadMountedDisplayFunctionLibrary.SetTrackingOrigin` "Floor" :!label _label))
    (:`SteamVR`
      (goto _label))
    (:`PSVR`
      (`HeadMountedDisplayFunctionLibrary.SetTrackingOrigin` "Eye")))
  (`SceneComponent.K2_AddLocalOffset` (`self.VROrigin`) (`KismetMathLibrary.MakeVector` 0.0 0.0 (`self.HeightCharacter`)) false false))

(event `InputAction|LeftTrigger`
  (params (Key :type "Key Structure"))
  (bind _leftinteract (`self.LeftInteract`))
  ;[1 1 1] Tiggers
  (:`Pressed`
    (if (`self.bWidget?`)
      (`WidgetInteractionComponent.PressPointerKey` _leftinteract "LeftMouseButton")
      (else
        (set `self.LeftTrigger?` true))))
  (:`Released`
    (`WidgetInteractionComponent.ReleasePointerKey` _leftinteract "LeftMouseButton")))

(event `InputAction|RightTrigger`
  (params (Key :type "Key Structure"))
  (bind _rightinteract (`self.RightInteract`))
  ;[1 1 1] Tiggers
  (:`Pressed`
    (if (`self.bWidget?`)
      (`WidgetInteractionComponent.PressPointerKey` _rightinteract "LeftMouseButton")
      (else
        (set `self.LeftTrigger?` false))))
  (:`Released`
    (`WidgetInteractionComponent.ReleasePointerKey` _rightinteract "LeftMouseButton")))

(event `self.ReceiveTick`
  (params (DeltaSeconds :type "Float (single-precision)"))
  (`self.LineTrace`))

(event `InputAxis|MoveForward`
  (params (AxisValue :type "Float (single-precision)"))
  (`self.AddMovementInput` (`KismetMathLibrary.MakeVector` (.x (`SceneComponent.GetForwardVector` (`self.Camera`))) (.y (`SceneComponent.GetForwardVector` (`self.Camera`)))) (* AxisValue (`self.MovementSpeed`))))

(event `InputAxis|MoveRight`
  (params (AxisValue :type "Float (single-precision)"))
  (`self.AddMovementInput` (`KismetMathLibrary.MakeVector` (.x (`SceneComponent.GetRightVector` (`self.Camera`))) (.y (`SceneComponent.GetRightVector` (`self.Camera`)))) (* AxisValue (`self.MovementSpeed`))))

(fn `LineTrace`
  (bind (_out_hit_bblockinghit _out_hit_binitialoverlap _out_hit_time _out_hit_distance _out_hit_location _out_hit_impactpoint _out_hit_normal _out_hit_impactnormal _out_hit_physmat _out_hit_hitactor) (`GameplayStatics.BreakHitResult` (`self.Out Hit`)))
  (bind _returnvalue (select `bool` (`self.LeftTrigger?`) :`false` (`self.RightInteract`) :`true` (`self.LeftInteract`) :!type "SceneComponent Object Reference"))
  (bind _returnvalue_2 (`SceneComponent.K2_GetComponentLocation` _returnvalue))
  (bind (_outhit _returnvalue_3) (`KismetSystemLibrary.LineTraceSingleForObjects` :`Start` _returnvalue_2 :`End` (+ _returnvalue_2 (* (`SceneComponent.GetForwardVector` _returnvalue) 300.0)) :`ObjectTypes` (`|MakeArray` "ObjectTypeQuery7" :!type "EObjectTypeQuery Enum") :`DrawDebugType` "ForOneFrame"))
  (set `self.Out Hit` _outhit)
  (set `self.bWidget?` _returnvalue_3)
  (if (not (`self.bWidget?`))
    (`WidgetInteractionComponent.ReleasePointerKey` (select `bool` (`self.LeftTrigger?`) :`false` (`self.RightInteract`) :`true` (`self.LeftInteract`)) "LeftMouseButton")
    (bind _asinstruction_widget (cast `/Game/Blueprint/Actor/Instruction_Widget` _out_hit_hitactor)
      (:`then`
        (`/Game/Blueprint/Actor/Instruction_Widget.HideWidget` _asinstruction_widget))
      (:`CastFailed`
        _)))
  (`ActorComponent.SetActive` (select `bool` (`self.LeftTrigger?`) :`false` (`self.RightInteract`) :`true` (`self.LeftInteract`)) (`self.bWidget?`) false)
  (`SceneComponent.SetVisibility` (select `bool` (`self.LeftTrigger?`) :`false` (`self.RightRedLine`) :`true` (`self.LeftRedLine`)) (`self.bWidget?`) true)
  (`SceneComponent.K2_SetWorldLocation` (select `bool` (`self.LeftTrigger?`) :`false` (`self.RightRedDot`) :`true` (`self.LeftRedDot`)) _out_hit_location false false)
  (return))

(fn `UserConstructionScript`)