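; VR player pawn that sets tracking origin per headset and scores hits on MasterTarget actors.
; Tick plays a whoop once each time Sphere's physics speed crosses a threshold.
; Capsule overlaps above that same Sphere speed trigger the target's hit and increment CutchDucks.
; Grab and release functions use the VR_InteractActor interface, but grab calls and thumbstick-style movement are disconnected, and SetAnimation is empty.
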(event `self.ReceiveBeginPlay`
  ;[1 1 1] FloorLevel
  (switch `name` (`HeadMountedDisplayFunctionLibrary.GetHMDDeviceName`)
    (:`Oculus Rift`
      (`HeadMountedDisplayFunctionLibrary.SetTrackingOrigin` "Floor" :!label _label))
    (:`SteamVR`
      (goto _label))
    (:`PSVR`
      (`HeadMountedDisplayFunctionLibrary.SetTrackingOrigin` "Eye")))
  (`SceneComponent.K2_AddLocalOffset` (`self.VROrigin`) (`KismetMathLibrary.MakeVector` 0.0 0.0 (`self.HeightCharacter`)) false false))

(event `self.ReceiveTick`
  (params (DeltaSeconds :type "Float (single-precision)"))
  (bind _returnvalue (`PrimitiveComponent.GetPhysicsLinearVelocity` (`self.Sphere`) "None"))
  (if (> (`KismetMathLibrary.VSize` _returnvalue) 900.0)
    (`/Engine/EditorBlueprintResources/StandardMacros.DoOnce` false :!label _label_2
      (:`Completed`
        (`GameplayStatics.PlaySound2D` "/Game/Assets/Sounds/243468__mark_ian__whoop__mp3cut_net__Cue.243468__mark_ian__whoop__mp3cut_net__Cue" 1.0 1.0 0.0 null null)))
    (else
      (goto _label_2 :!via `Reset`))))

(event `InputAction|LeftGrip`
  (params (Key :type "Key Structure")))

(event `InputAction|RightGrip`
  (params (Key :type "Key Structure")))

(event `InputAxis|MoveForward`
  (params (AxisValue :type "Float (single-precision)")))

(event `InputAxis|MoveRight`
  (params (AxisValue :type "Float (single-precision)")))

(event `self.Capsule.OnComponentBeginOverlap`
  (params (OverlappedComponent :type "PrimitiveComponent Object Reference") (OtherActor :type "Actor Object Reference") (OtherComp :type "PrimitiveComponent Object Reference") (OtherBodyIndex :type Integer) (bFromSweep :type Boolean) (SweepResult :type "HitResult Structure (by ref)"))
  (bind _asmaster_target (cast `/Game/Blueprint/Actor/MasterTarget` OtherActor))
  (bind _returnvalue (`PrimitiveComponent.GetPhysicsLinearVelocity` (`self.Sphere`) "None"))
  (if (> (`KismetMathLibrary.VSize` _returnvalue) 900.0)
    (`/Game/Blueprint/Actor/MasterTarget.GetHit` _asmaster_target)
    (bind _result (`/Engine/EditorBlueprintResources/StandardMacros.IncrementInt` (`self.CutchDucks`))
      (:`  `
        (set `self.CutchDucks` _result)))))

(fn `ActorNearHand`
  (params (Hand :type "/Game/Blueprint/Other/Enum/Enum_Hands Enum" :default "NewEnumerator0"))
  (returns (Interact_Actor :type "Actor Object Reference"))
  (locals (InteractActor :type "Actor Object Reference"))
  (for _array_element (`PrimitiveComponent.GetOverlappingActors` (select `/Game/Blueprint/Other/Enum/Enum_Hands` Hand :!type "PrimitiveComponent Object Reference") null)
    (if (`KismetSystemLibrary.DoesImplementInterface` _array_element "/Game/Blueprint/Other/Interface/VR_InteractActor.VR_InteractActor_C")
      (set `local.InteractActor` _array_element)))
  (return (`local.InteractActor`)))

(fn `GrabActor`
  (params (Hand :type "/Game/Blueprint/Other/Enum/Enum_Hands Enum" :default "NewEnumerator0"))
  (bind _hand (`local.Hand`))
  (bind _interact_actor (`self.ActorNearHand` Hand))
  (`/Engine/EditorBlueprintResources/StandardMacros.IsValid` _interact_actor
    (:`Is Valid`
      (bind _output_get (set `self.AttachedActor` _interact_actor))
      (message `/Game/Blueprint/Other/Interface/VR_InteractActor.Grab` _output_get (select `/Game/Blueprint/Other/Enum/Enum_Hands` _hand :!type "SceneComponent Object Reference"))
      (`self.SetAnimation` _hand "/Game/Assets/Models/Hands/Animations/Grab_Hand.Grab_Hand")
      (return))))

(fn `ReleaseActor`
  (params (Hand :type "/Game/Blueprint/Other/Enum/Enum_Hands Enum" :default "NewEnumerator0"))
  (if (== (select `/Game/Blueprint/Other/Enum/Enum_Hands` Hand :`NewEnumerator0` (`self.RightHand_Controller`) :`NewEnumerator1` (`self.LeftHand_Controller`)) (`SceneComponent.GetAttachParent` (`Actor.RootComponent` (`self.AttachedActor`))))
    (message `/Game/Blueprint/Other/Interface/VR_InteractActor.Drop` (`self.AttachedActor`))
    (set `self.AttachedActor` null)
    (`self.SetAnimation` Hand "/Game/Assets/Models/Hands/Animations/Idle_Hand.Idle_Hand")
    (return)
    (else
      (return))))

(fn `SetAnimation`
  (params (Selection :type "/Game/Blueprint/Other/Enum/Enum_Hands Enum" :default "NewEnumerator0") (NewAnimToPlay :type "AnimationAsset Object Reference")))

(fn `UserConstructionScript`)