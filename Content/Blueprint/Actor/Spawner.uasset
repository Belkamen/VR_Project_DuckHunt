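; Spawner actor that spawns duck targets on the level's spline paths through its SpawnDucks event.
; Each call picks a random SplineDirection actor and spawns a MasterTarget AI at its location, facing along the spawner's Arrow component.
; It then assigns that spline actor to the new target's Spline variable.
; Nothing in this file calls SpawnDucks, and an unused SpawnActor node remains disconnected.
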(event `SpawnDucks`
  (bind _outactors (`GameplayStatics.GetAllActorsOfClass` "/Game/Blueprint/Actor/SplineDirection.SplineDirection_C"))
  (set `self.Index` (`KismetMathLibrary.RandomInteger` (`KismetArrayLibrary.Array_Length` _outactors)))
  (bind _output (`|GetArrayItem` _outactors (`self.Index`)))
  (bind _returnvalue (`AIBlueprintHelperLibrary.SpawnAIFromClass` "/Game/Blueprint/Actor/MasterTarget.MasterTarget_C" null (`self.K2_GetActorLocation` _output) (`SceneComponent.K2_GetComponentRotation` (`self.Arrow`)) false null))
  (bind _asmaster_target (cast `/Game/Blueprint/Actor/MasterTarget` _returnvalue))
  (set `/Game/Blueprint/Actor/MasterTarget.Spline` _output _asmaster_target))

(fn `UserConstructionScript`)