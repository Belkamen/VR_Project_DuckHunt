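; Manager actor that keeps spawning duck targets by periodically triggering random Spawner actors.
; A looping timer starts on BeginPlay or Interact, with its interval randomized when it is set.
; Each tick of the timer counts MasterTarget actors and, while they are below Amount, calls SpawnDucks on a randomly chosen Spawner.
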(event `self.ReceiveBeginPlay`
  (`KismetSystemLibrary.K2_SetTimerDelegate` (delegate `CustomEvent_0`) (`KismetMathLibrary.RandomFloatInRange` 0.7 3.0) true :!label _label))

(event `/Game/Blueprint/Other/Interface/VR_InteractActor.Interact`
  (goto _label))

(event `CustomEvent_0`
  (bind _outactors (`GameplayStatics.GetAllActorsOfClass` "/Game/Blueprint/Actor/MasterTarget.MasterTarget_C"))
  (if (not (>= (`KismetArrayLibrary.Array_Length` _outactors) (`self.Amount`)))
    (bind _outactors_2 (`GameplayStatics.GetAllActorsOfClass` "/Game/Blueprint/Actor/Spawner.Spawner_C"))
    (`/Game/Blueprint/Actor/Spawner.SpawnDucks` (`|GetArrayItem` _outactors_2 (`KismetMathLibrary.RandomInteger` (`KismetArrayLibrary.Array_Length` _outactors_2))))))

(fn `UserConstructionScript`)