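; Main menu door actor that opens and loads the level named in LevelName when interacted with.
; On BeginPlay it registers itself as Owner of the OpenDoor widget in its Widget component.
; Interact skips an unset LevelName; otherwise a timeline swings the door mesh open.
; When the timeline finishes, the camera cuts to solid white via manual fade, then the level loads after a short delay.
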(event `self.ReceiveBeginPlay`
  (bind _asopen_door (cast `/Game/Blueprint/OpenDoor` (`WidgetComponent.GetUserWidgetObject` (`self.Widget`))))
  (set `/Game/Blueprint/OpenDoor.Owner` self _asopen_door))

(event `OpenDoor`
  (bind (_direction _alpha) (`Timeline|Alpha` :!via `PlayFromStart`)
    (:`Update`
      (`SceneComponent.K2_SetRelativeRotation` (`self.Urasa_Brusok_dlya_DVERI10`) (`KismetMathLibrary.RLerp` (struct) (struct :`Yaw` 90.0) _alpha) false false))
    (:`Finished`
      (`PlayerCameraManager.SetManualCameraFade` (`PlayerController.PlayerCameraManager` (`GameplayStatics.GetPlayerController` 0)) 1.0 (struct :`R` 1.0 :`G` 1.0 :`B` 1.0 :`A` 1.0) false)
      (`KismetSystemLibrary.Delay` 1.0)
      (`GameplayStatics.OpenLevel` (`self.Level Name`)))))

(event `/Game/Blueprint/Other/Interface/VR_InteractActor.Interact`
  (if (not (== (`self.Level Name`) "None"))
    (`self.OpenDoor`)))

(fn `UserConstructionScript`)