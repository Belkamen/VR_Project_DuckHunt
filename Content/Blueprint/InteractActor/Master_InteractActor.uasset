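; Master interact actor that can be picked up by a hand component and dropped, apparently as a base for grabbable objects.
; Grab stores the given component and, for the first hand only, turns off mesh physics, snaps the mesh to it and applies a one-hand rotation.
; Drop re-enables physics, detaches the mesh and resets the first-hand flag.
; Later grabs only update the stored attach component, with no two-hand handling.
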(event `/Game/Blueprint/Other/Interface/VR_InteractActor.Grab`
  (params (AttachTo :type "SceneComponent Object Reference"))
  (set `self.AttachComponent` AttachTo)
  (if (`self.IsFirstHand?`)
    (`PrimitiveComponent.SetSimulatePhysics` (`self.Mesh`) false)
    (`SceneComponent.K2_AttachToComponent` (`self.Mesh`) (`self.AttachComponent`) "None" "SnapToTarget" "SnapToTarget" "KeepRelative" true)
    (`SceneComponent.K2_SetRelativeRotation` (`self.Mesh`) (`self.OneHandRotation`) false false)
    (set `self.IsFirstHand?` false)
    (set `self.FirstHand` (`self.AttachComponent`))))

(event `/Game/Blueprint/Other/Interface/VR_InteractActor.Drop`
  (bind _mesh (`self.Mesh`))
  (`PrimitiveComponent.SetSimulatePhysics` _mesh true)
  (`SceneComponent.K2_DetachFromComponent` _mesh "KeepRelative" "KeepRelative" "KeepRelative" true)
  (set `self.IsFirstHand?` true))

(fn `UserConstructionScript`)